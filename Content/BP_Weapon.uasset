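; BP_Weapon is an axe weapon actor that a character can hold and release through interaction events.
; On hold, it disables physics and collision on the axe mesh, then snaps it to a socket on the character's mesh with a configurable relative offset.
; Only the mesh component is attached, and non-Character holders stop the event after physics and collision are already off.
; On detach, it restores physics and collision and releases the mesh at its world transform.
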(event EventActorInteractHold
  (params (ActorToHold :type Actor%20Object%20Reference))
  (bind _sm_axe_01 (Variables|Default|GetSM_Axe_01))
  (Physics|SetSimulatePhysics _sm_axe_01 false)
  (Collision|SetCollisionEnabled _sm_axe_01 "NoCollision")
  (bind _ascharacter (Utilities|Casting|CastToCharacter ActorToHold))
  (Transformation|AttachComponentToComponent _sm_axe_01 (Variables|/Script/Engine.Character|GetMesh _ascharacter) (Variables|Default|GetHoldSocketName) "SnapToTarget" "SnapToTarget" "KeepRelative" true)
  (Transformation|SetRelativeLocationAndRotation _sm_axe_01 (Variables|Default|GetHoldRelativeLocation) (Variables|Default|GetHoldRelativeRotation) false false))

(event EventActorInteractDetach
  (params (ActorToHold :type Actor%20Object%20Reference))
  (bind _sm_axe_01 (Variables|Default|GetSM_Axe_01))
  (Physics|SetSimulatePhysics _sm_axe_01 true)
  (Collision|SetCollisionEnabled _sm_axe_01 "QueryAndPhysics")
  (Transformation|DetachFromComponent _sm_axe_01 "KeepWorld" "KeepWorld" "KeepRelative" true))

(fn ConstructionScript)