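; BP_InnSimilatorLibrary is a Blueprint function library for the inn simulator that builds randomized NPC body appearances.
; Its single function picks one of two numbered rows in DT_NPC_Characters by converting a random integer to a row name.
; It then draws independently from that row's part arrays and returns head, hair, hat, chest, arm and leg.
; Only the row-found branch is wired to a return.
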(fn FLRandomBodyforNPC
  (bind _returnvalue (Utilities|GetDataTableRow "/Game/InnSimilator/Blueprints/Data/DT_NPC_Characters.DT_NPC_Characters" (Utilities|String|StringToName (Utilities|String|ToString(Integer) (Math|Random|RandomIntegerinRange 0 1))))
    (:then
      (return (Utilities|MLRandomfromArray (.Head (Utilities|Struct|BreakS_CharacterStructs _returnvalue))) (Utilities|MLRandomfromArray (.Hair (Utilities|Struct|BreakS_CharacterStructs _returnvalue))) (Utilities|MLRandomfromArray (.Hat (Utilities|Struct|BreakS_CharacterStructs _returnvalue))) (Utilities|MLRandomfromArray (.Chest (Utilities|Struct|BreakS_CharacterStructs _returnvalue))) (Utilities|MLRandomfromArray (.Arm (Utilities|Struct|BreakS_CharacterStructs _returnvalue))) (Utilities|MLRandomfromArray (.Leg (Utilities|Struct|BreakS_CharacterStructs _returnvalue)))))))