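; BP_InnPlayer is the player character Blueprint for the inn simulator, handling held items and arm animation input.
; It sets holding and arm-forward flags on ABP_InnSimilatorPlayer at begin play and on right mouse, while Q detaches the held item.
; Use plays an attack montage when the held InteractActorCore's type is Use.
; Tick debug-prints whether SeenActor implements SInteractInterface; the local interact trace function is empty.
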(event EventTick
  (params (DeltaSeconds :type Float%20%28single-precision%29))
  (Development|PrintString (Utilities|String|ToString(Boolean) (Utilities|DoesObjectImplementInterface (Variables|Default|GetSeenActor) "/Script/GameplayPlugin.SInteractInterface")) true true "(R=0.000000,G=0.660000,B=1.000000,A=1.000000)" 0.0))

(event Collision|EventActorBeginOverlap
  (params (OtherActor :type Actor%20Object%20Reference)))

(event EventBeginPlay
  (Variables|/Game/InnSimilator/Blueprints/Player/ABP_InnSimilatorPlayer.ABP_InnSimilatorPlayer_C|SetbIsHoldingSomething (CallFunction|FGetAnimBlueprint) true))

(event Input|ActionEvents|InputActionUse
  (params (Key :type Key%20Structure :default "None"))
  (:Pressed
    (bind _asinteract_actor_core (Utilities|Casting|CastToInteractActorCore (Variables|Default|GetItemInHand)))
    (switch Utilities|FlowControl|Switch|SwitchonInteractType (Variables|/Script/GameplayPlugin.InteractActorCore|GetActorInteractType _asinteract_actor_core)
      (:Use
        (Animation|Montage|PlayMontage (Variables|Character|GetMesh) "/Game/Marketplace/ModularMedievalNPC/DemoContent/Animations/ThirdPersonIdleHoldAttack_Montage.ThirdPersonIdleHoldAttack_Montage")))))

(event Input|KeyboardEvents|Q
  (params (Key :type Key%20Structure :default "None"))
  (:Pressed
    (Class|SPlayer|DetachIteminHand)))

(event Input|MouseEvents|RightMouseButton
  (params (Key :type Key%20Structure :default "None"))
  (bind _asabp_inn_similator_player (CallFunction|FGetAnimBlueprint))
  (:Pressed
    (Variables|/Game/InnSimilator/Blueprints/Player/ABP_InnSimilatorPlayer.ABP_InnSimilatorPlayer_C|SetArmForward _asabp_inn_similator_player true))
  (:Released
    (Variables|/Game/InnSimilator/Blueprints/Player/ABP_InnSimilatorPlayer.ABP_InnSimilatorPlayer_C|SetArmForward _asabp_inn_similator_player false)))

(fn ConstructionScript)

(fn FTraceforInteract)

(fn FGetAnimBlueprint
  (bind _asabp_inn_similator_player (Utilities|Casting|CastToABP_InnSimilatorPlayer (Components|SkeletalMesh|GetAnimInstance (Variables|Character|GetMesh))))
  (return _asabp_inn_similator_player))