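; BP_GoldPocket is a gold pouch actor that a character can pick up, carry and drop.
; The hold event disables physics and collision on the sack mesh, then snaps it to a named socket on the holding character's mesh.
; The detach event restores physics and collision and releases the mesh at its current world transform.
; Only the mesh component is attached, not the actor itself.
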(event EventActorInteractHold
  (params (ActorToHold :type Actor%20Object%20Reference))
  (bind _sm_sac (Variables|Default|GetSM_sac))
  (Physics|SetSimulatePhysics _sm_sac false)
  (Collision|SetCollisionEnabled _sm_sac "NoCollision")
  (bind _ascharacter (Utilities|Casting|CastToCharacter ActorToHold))
  (Transformation|AttachComponentToComponent _sm_sac (Variables|/Script/Engine.Character|GetMesh _ascharacter) (Variables|Default|GetHoldSocketName) "SnapToTarget" "SnapToTarget" "KeepRelative" true))

(event EventActorInteractDetach
  (params (ActorToHold :type Actor%20Object%20Reference))
  (bind _sm_sac (Variables|Default|GetSM_sac))
  (Physics|SetSimulatePhysics _sm_sac true)
  (Collision|SetCollisionEnabled _sm_sac "QueryAndPhysics")
  (Transformation|DetachFromComponent _sm_sac "KeepWorld" "KeepWorld" "KeepRelative" true))

(fn ConstructionScript)