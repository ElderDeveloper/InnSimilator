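; Shop actor for the inn simulator that manages a queue of waiting NPCs at offsets defined in WaitLine, previewed as billboards.
; Functions find the first free slot, then reserve it for an NPC and return its location and rotation facing the shop.
; The first-in-line NPC's request is cached; box overlaps compare incoming actors against its class and tag, currently only printing debug output, as does Tick.
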(event OnComponentBeginOverlap(Box)
  (params (OverlappedComponent :type Primitive%20Component%20Object%20Reference) (OtherActor :type Actor%20Object%20Reference) (OtherComp :type Primitive%20Component%20Object%20Reference) (OtherBodyIndex :type Integer) (bFromSweep :type Boolean) (SweepResult :type Hit%20Result%20Structure%20%28by%20ref%29))
  (bind _ai_requestfirstinline (Variables|Default|GetAI_RequestFirstInLine))
  (if (and (== (Utilities|GetClass OtherActor) (.actorreferance _ai_requestfirstinline)) (!= (Utilities|Array|FindItem (Variables|/Script/Engine.Actor|GetTags OtherActor) (.tag _ai_requestfirstinline)) -1))
    (Development|PrintString "Hello" true true "(R=1.000000,G=0.000000,B=0.066279,A=1.000000)" 1e+01)
    (else
      (Development|PrintString (Utilities|GetDisplayName OtherActor)))))

(event EventBeginPlay)

(event Collision|EventActorBeginOverlap
  (params (OtherActor :type Actor%20Object%20Reference)))

(event EventTick
  (params (DeltaSeconds :type Float%20%28single-precision%29))
  (bind _ai_requestfirstinline (Variables|Default|GetAI_RequestFirstInLine))
  (Development|PrintString (Utilities|String|ToString(Text) (Utilities|Text|FormatText "{a}  |   {b}" (Utilities|Text|ToText(String) (Utilities|GetClassDisplayName (.actorreferance _ai_requestfirstinline))) (Utilities|Text|ToText(Name) (.tag _ai_requestfirstinline)))) true true "(R=0.000000,G=0.660000,B=1.000000,A=1.000000)" 0.0))

(fn ConstructionScript
  (Utilities|Array|Resize (Variables|Default|GetLineIndexOcuppied) (Utilities|Array|Length (Variables|Default|GetWaitLine)))
  (for _array_element (Variables|Default|GetWaitLine)
    (AddComponent|AddBillboardComponent false (Math|Transform|MakeTransform _array_element "0, 0, 0" "0.280000,0.280000,0.280000")))
  (Transformation|SetRelativeScale3D (Variables|Default|GetBox) (Variables|Default|GetBoxScale))
  (Utilities|Array|Resize (Variables|Default|GetWaitingNPC) (Utilities|Array|Length (Variables|Default|GetWaitLine))))

(fn FRequestEmptyLine
  (bind (_array_element _array_index) (Utilities|Array|ForEachLoopwithBreak (Variables|Default|GetLineIndexOcuppied) :!label _label)
    (:LoopBody
      (if (Math|Boolean|Equal(Boolean) _array_element false)
        (LocalVariables|SetFoundIndx _array_index)
        (Utilities|FlowControl|Sequence
          (:then_0
            (goto _label Break))
          (:then_1
            (return true (LocalVariables|GetFoundIndx))))))
    (:Completed
      (return false -1))))

(fn FRequestLineLocationandTurnRotation
  (params (IndexToTest :type Integer) (Npc :type BP%20S%20Core%20Npc%20Object%20Reference))
  (bind _returnvalue (Transformation|GetActorLocation))
  (bind _waitline (Variables|Default|GetWaitLine))
  (if (Utilities|Array|IsValidIndex _waitline IndexToTest)
    (bind _output_get (LocalVariables|SetLocalLocation (+ _returnvalue (Utilities|Array|Get(acopy) _waitline IndexToTest))))
    (Utilities|Array|SetArrayElem (Variables|Default|GetLineIndexOcuppied) IndexToTest true)
    (CallFunction|FControlAllFull)
    (Utilities|Array|SetArrayElem (Variables|Default|GetWaitingNPC) IndexToTest Npc)
    (CallFunction|FGetAIRequest)
    (return true _output_get (Math|Rotator|FindLookatRotation (LocalVariables|GetLocalLocation) _returnvalue))
    (else
      (return false "0, 0, 0" "0, 0, 0"))))

(fn FControlAllFull
  (bind _array_element (Utilities|Array|ForEachLoopwithBreak (Variables|Default|GetLineIndexOcuppied) :!label _label)
    (:LoopBody
      (if (not (Math|Boolean|Equal(Boolean) _array_element true))
        (Utilities|FlowControl|Sequence
          (:then_0
            (goto _label Break))
          (:then_1
            (Variables|Default|SetbAllSlotsFull true)))))))

(fn FGetAIRequest
  (bind _waitingnpc (Variables|Default|GetWaitingNPC))
  (if (Utilities|Array|IsValidIndex _waitingnpc)
    (Variables|Default|SetAI_RequestFirstInLine (Variables|/Game/InnSimilator/Blueprints/AI/BP_SCoreNpc.BP_SCoreNpc_C|GetS_Request (Utilities|Array|Get(acopy) _waitingnpc)))))