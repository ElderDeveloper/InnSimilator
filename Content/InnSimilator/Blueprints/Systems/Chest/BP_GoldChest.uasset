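; Gold chest that banks gold pockets for the player and swings its lid open while the player is nearby.
; A proximity sphere plays and reverses a timeline that drives lid rotation through the chest's Anim Blueprint.
; The inside trigger converts overlapping gold pockets into player gold with sound and particles, then destroys them.
; Other non-player objects entering it get their overlapping component teleported to a random point in TransformBox.
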(event OnComponentBeginOverlap(Inside)
  (params (OverlappedComponent :type Primitive%20Component%20Object%20Reference) (OtherActor :type Actor%20Object%20Reference) (OtherComp :type Primitive%20Component%20Object%20Reference) (OtherBodyIndex :type Integer) (bFromSweep :type Boolean) (SweepResult :type Hit%20Result%20Structure%20%28by%20ref%29))
  (bind _newgold (Variables|Default|GetNewGold))
  (bind _transformbox (Variables|Default|GetTransformBox))
  (if (Utilities|DoesObjectImplementInterface OtherActor "/Script/GameplayPlugin.SInteractInterface")
    (bind _asbp_gold_pocket (Utilities|Casting|CastToBP_GoldPocket OtherActor)
      (:then
        (Class|SInnSimilatorLibrary|AddGoldtoPlayer (Variables|/Game/InnSimilator/Blueprints/Systems/Gold/BP_GoldPocket.BP_GoldPocket_C|GetGoldAmount _asbp_gold_pocket))
        (Actor|DestroyActor _asbp_gold_pocket)
        (Audio|PlaySound2D (Variables|Default|GetGoldColletSound) 1.0 1.0 0.0 0 0)
        (Effects|Components|ParticleSystem|SetTemplate _newgold (Variables|Default|GetGoldColletEmitter))
        (Components|Activation|Activate _newgold true))
      (:CastFailed
        (Transformation|SetWorldLocation OtherComp (Math|Random|RandomPointinBoundingBox (Transformation|GetWorldLocation _transformbox) (Variables|/Script/Engine.BoxComponent|GetBoxExtent _transformbox)) false false :!label _label)))
    (elif (not (Utilities|DoesObjectImplementInterface OtherActor "/Script/GameplayPlugin.SPlayerInterface"))
      (goto _label))))

(event OnComponentBeginOverlap(Sphere)
  (params (OverlappedComponent :type Primitive%20Component%20Object%20Reference) (OtherActor :type Actor%20Object%20Reference) (OtherComp :type Primitive%20Component%20Object%20Reference) (OtherBodyIndex :type Integer) (bFromSweep :type Boolean) (SweepResult :type Hit%20Result%20Structure%20%28by%20ref%29))
  (if (Utilities|DoesObjectImplementInterface OtherActor "/Script/GameplayPlugin.SPlayerInterface")
    (bind _newtrack_0 (Timeline|Chest Play)
      (:Update
        (Variables|/Game/InnSimilator/Blueprints/Systems/Chest/Chest09_animated_Skeleton_AnimBlueprint.Chest09_animated_Skeleton_AnimBlueprint_C|SetRotation (Variables|Default|GetAnimBP) (Math|Float|Lerp 0.0 -115.0 _newtrack_0))))))

(event OnComponentEndOverlap(Sphere)
  (params (OverlappedComponent :type Primitive%20Component%20Object%20Reference) (OtherActor :type Actor%20Object%20Reference) (OtherComp :type Primitive%20Component%20Object%20Reference) (OtherBodyIndex :type Integer))
  (if (Utilities|DoesObjectImplementInterface OtherActor "/Script/GameplayPlugin.SPlayerInterface")
    (bind _newtrack_0 (Timeline|Chest Reverse)
      (:Update
        (Variables|/Game/InnSimilator/Blueprints/Systems/Chest/Chest09_animated_Skeleton_AnimBlueprint.Chest09_animated_Skeleton_AnimBlueprint_C|SetRotation (Variables|Default|GetAnimBP) (Math|Float|Lerp 0.0 -115.0 _newtrack_0))))))

(event EventBeginPlay
  (bind _aschest_09_animated_skeleton_anim_blueprint (Utilities|Casting|CastToChest09_animated_Skeleton_AnimBlueprint (Components|SkeletalMesh|GetAnimInstance (Variables|Default|GetChest09_animated))))
  (Variables|Default|SetAnimBP _aschest_09_animated_skeleton_anim_blueprint))

(fn ConstructionScript)