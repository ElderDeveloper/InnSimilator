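; Core NPC Blueprint for the inn simulator that handles requests to queue at a shop.
; On the first successful request, it gets a line location and turn rotation from the shop controller for the given wait index.
; It writes these, the shop reference and a new AI state to the blackboard through a helper, then sets a flag that blocks further requests.
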(event Custom|ReceiveShopRequest
  (params (ShopController :type BP%20Shop%20and%20Wait%20Line%20Object%20Reference) (WaitIndex :type Integer))
  (bind (_returnvalue _nameout) (CallFunction|FGetBlackboard "AiState"))
  (bind (_returnvalue_2 _nameout_2) (CallFunction|FGetBlackboard "ShopRotation"))
  (bind (_returnvalue_3 _nameout_3) (CallFunction|FGetBlackboard "ShopReferance"))
  (bind (_returnvalue_4 _nameout_4) (CallFunction|FGetBlackboard "ShopLocation"))
  (if (not (Variables|Default|GetbHasReceivedRequest))
    (bind (_bsuccess _location _rotation) (Default|FRequestLineLocationandTurnRotation ShopController WaitIndex self))
    (if _bsuccess
      (AI|Components|Blackboard|SetValueasVector _returnvalue_4 _nameout_4 _location)
      (Class|BlackboardComponent|SetValueasRotator _returnvalue_2 _nameout_2 _rotation)
      (AI|Components|Blackboard|SetValueasObject _returnvalue_3 _nameout_3 ShopController)
      (bind _output_get (Variables|Default|SetAiState "NewEnumerator4"))
      (AI|Components|Blackboard|SetValueasEnum _returnvalue _nameout _output_get)
      (Variables|Default|SetbHasReceivedRequest true))))

(event EventBeginPlay
  (|CallParentFunction) ; This node is disabled and will not be called.\nDrag off pins to build functionality.
)

(fn ConstructionScript
  (|CallParentFunction))

(fn FGetBlackboard
  (params (NameIn :type Name))
  (return (AI|GetBlackboard self) NameIn))