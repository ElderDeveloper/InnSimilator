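; BP_InnSimilatorCore is the central coordinator for an inn simulation, directing NPCs to shops and social spots.
; On BeginPlay it gathers all shop lines, social task locations and NPCs, then starts a looping timer.
; Each tick of that timer picks a random shop and, if it has an empty line slot, sends a random NPC there.
; A separate function reserves and returns a random free social point using a parallel occupancy array.
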(event EventBeginPlay
  (Utilities|FlowControl|Sequence
    (:then_0
      (bind _outactors (Actor|GetAllActorsOfClass "/Game/InnSimilator/Blueprints/Systems/WorldCotrollers/Shop/BP_ShopAndWaitLine.BP_ShopAndWaitLine_C"))
      (Variables|Default|SetShopWaitAndBuyLine _outactors))
    (:then_1
      (bind _outactors_2 (Actor|GetAllActorsOfClass "/Game/InnSimilator/Blueprints/Systems/WorldCotrollers/SocialEvents/BP_AISocialTask.BP_AISocialTask_C"))
      (Variables|Social|SetSocialTaskLocations _outactors_2))
    (:then_2
      (Utilities|Array|Resize (Variables|Social|GetSocialTaskLocationsOcuppied) (Utilities|Array|Length (Variables|Social|GetSocialTaskLocations))))
    (:then_3
      (bind _outactors_3 (Actor|GetAllActorsOfClass "/Game/InnSimilator/Blueprints/AI/BP_SCoreNpc.BP_SCoreNpc_C"))
      (Variables|Default|SetAllNPC _outactors_3))
    (:then_4
      (Utilities|Time|SetTimerbyFunctionName 0 "F_SendAiToShop" 1.0 true))))

(fn ConstructionScript)

(fn FFindRandomSocialPoint
  (bind _indexes (LocalVariables|GetIndexes))
  (for (_array_element _array_index) (Variables|Social|GetSocialTaskLocationsOcuppied)
    (if (not _array_element)
      (Utilities|Array|Add (LocalVariables|GetIndexes) _array_index)))
  (if (> (Utilities|Array|Length _indexes) 0)
    (LocalVariables|SetSelectedIndex (Utilities|MLRandomfromArray _indexes))
    (Utilities|Array|SetArrayElem (Variables|Social|GetSocialTaskLocationsOcuppied) (LocalVariables|GetSelectedIndex) true)
    (return true (Utilities|Array|Get(acopy) (Variables|Social|GetSocialTaskLocations) (LocalVariables|GetSelectedIndex)) (LocalVariables|GetSelectedIndex))
    (else
      (return false 0 -1))))

(fn FSendAitoShop
  (bind _output_get (LocalVariables|SetLocalShop (Utilities|MLRandomfromArray (Variables|Default|GetShopWaitAndBuyLine))))
  (bind (_found _lineindex) (Default|FRequestEmptyLine _output_get))
  (if _found
    (Default|ReceiveShopRequest (Utilities|MLRandomfromArray (Variables|Default|GetAllNPC)) (LocalVariables|GetLocalShop) _lineindex)))